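; BP_OSCIn is an actor that receives OSC data and visualizes it as rows of colored cubes.
; It starts an OSC server on BeginPlay and reads all floats from the first message of each received bundle.
; Each float spawns a new BP_Cube in a centered row relative to the actor.
; A dynamic material colors each cube by mapping its range-normalized value to hue.
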(event Custom|OnBundleReceived
  (params (Bundle :type OSC%20Bundle%20Structure%20%28by%20ref%29) (IPAddress :type String) (Port :type Integer))
  (bind _spacing (Variables|Default|GetSpacing))
  (bind _returnvalue (Class|OSCManager|GetMessagefromBundle Bundle))
  (bind _values (Class|OSCManager|GetAllFloats _returnvalue))
  (for (_array_element _array_index) _values
    (bind _returnvalue_2 (Game|SpawnActorfromClass "/Game/BP_Cube.BP_Cube_C" (Math|Transform|MakeRelativeTransform (Math|Conversions|ToTransform(Vector) (Math|Conversions|ToVector(Vector4) (Math|Vector4|MakeVector4 0.0 (- (* (Math|Conversions|ToFloat(Integer) _array_index) _spacing) (/ (* _spacing (- (Utilities|Array|Length _values) 1)) 2)) 1.5e+02 0.0))) (Transformation|GetActorTransform)) "Undefined" "MultiplyWithRoot" 0 0))
    (bind _returnvalue_3 (Rendering|Material|CreateDynamicMaterialInstance (Variables|/Game/BP_Cube.BP_Cube_C|GetCube _returnvalue_2) 0 0 "None" :!class /Script/Engine.PrimitiveComponent))
    (Rendering|Material|SetVectorParameterValue _returnvalue_3 "Base Color" (Class|KismetMathLibrary|HSVtoRGB (* (Math|Float|NormalizetoRange _array_element (Variables|Default|GetRange%20Min) (Variables|Default|GetRange%20Max)) 3.6e+02) 1.0 1.0 1.0) :!class /Script/Engine.MaterialInstanceDynamic)))

(event Collision|EventActorBeginOverlap
  (params (OtherActor :type Actor%20Object%20Reference)))

(event EventTick
  (params (DeltaSeconds :type Float%20%28single-precision%29)))

(event EventBeginPlay
  (bind _returnvalue (Class|OSCManager|CreateOSCServer (Variables|Default|GetReceive%20IPAddress) (Variables|Default|GetPort) false true "UE_OSC" 0))
  (bind _output_get (Variables|Default|SetServer _returnvalue))
  (EventDispatchers|BindEventtoOnOscBundleReceived _output_get (delegate Custom|OnBundleReceived)))

(fn ConstructionScript)