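; BP_Attactor drives a Niagara effect's user parameters from incoming OSC messages.
; An OSC receive event routes /volume values to user_alpha and /pitch values to user_beta.
; A disconnected branch that would send /pitch to user_rho never runs, and BeginPlay, overlap and Tick are empty.
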(event OnOscReceived(BP_OSCIn)
  (params (Address :type String) (Value :type String))
  (if (Utilities|Enum|Equal(Enum) Address "/volume")
    (Niagara|SetNiagaraVariable(Float) (Variables|Default|GetNiagara) "user_alpha" (Math|Conversions|ToFloat(Integer) Value))
    (elif (Utilities|Enum|Equal(Enum) Address "/pitch")
      (Niagara|SetNiagaraVariable(Float) (Variables|Default|GetNiagara) "user_beta" (Math|Conversions|ToFloat(Integer) Value)))))

(event EventBeginPlay)

(event Collision|EventActorBeginOverlap
  (params (OtherActor :type Actor%20Object%20Reference)))

(event EventTick
  (params (DeltaSeconds :type Float%20%28single-precision%29)))

(fn ConstructionScript)