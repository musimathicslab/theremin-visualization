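; BP_AudioParticles is an actor that drives a Niagara particle effect from incoming OSC messages, making it react to audio-style parameters.
; Its OSC receive event branches on the address and feeds scaled values into Niagara float variables.
; Volume trades attractor strength against noise strength and also sets the noiseNegative variable.
; Pitch drives vortex force, while the mul channel inversely controls drag.
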(event OnOscReceived(BP_OSCIn)
  (params (Address :type String) (Value :type String))
  (bind _returnvalue (Math|Conversions|ToFloat(Integer) Value))
  (bind _niagara (Variables|Default|GetNiagara))
  (bind _returnvalue_2 (* _returnvalue 7e+03))
  (if (Utilities|Enum|Equal(Enum) Address "/volume")
    (Niagara|SetNiagaraVariable(Float) _niagara "attrStrength" (* (- 1.0 _returnvalue) 5e+02))
    (Niagara|SetNiagaraVariable(Float) _niagara "noiseStrength" _returnvalue_2)
    (bind _result (Math|Float|NegateFloat _returnvalue_2)
      (:%20%20
        (Niagara|SetNiagaraVariable(Float) _niagara "noiseNegative" _result)))
    (elif (Utilities|Enum|Equal(Enum) Address "/pitch")
      (Niagara|SetNiagaraVariable(Float) (Variables|Default|GetNiagara) "vortexForce" (* (Math|Conversions|ToFloat(Integer) Value) 1e+03))
      (elif (Utilities|Enum|Equal(Enum) Address "/mul")
        (Niagara|SetNiagaraVariable(Float) (Variables|Default|GetNiagara) "drag" (* (- 1.0 (Math|Conversions|ToFloat(Integer) Value)) 2e+01))))))

(event EventBeginPlay)

(event Collision|EventActorBeginOverlap
  (params (OtherActor :type Actor%20Object%20Reference)))

(event EventTick
  (params (DeltaSeconds :type Float%20%28single-precision%29)))

(fn ConstructionScript)