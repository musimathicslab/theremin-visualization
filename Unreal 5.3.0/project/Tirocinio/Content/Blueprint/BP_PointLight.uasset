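; BP_PointLight is a point light actor whose color is driven remotely over OSC.
; A BP_OSCIn receive event checks the address for /r, /g or /b and stores the value in the matching channel variable.
; Each matching message then rebuilds the color from all three stored channels and applies it to the PointLight in sRGB.
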(event OnOscReceived(BP_OSCIn)
  (params (Address :type String) (Value :type String))
  (bind _returnvalue (Math|Conversions|ToFloat(Integer) Value))
  (if (Utilities|Enum|Equal(Enum) Address "/r")
    (Variables|Default|SetR _returnvalue)
    (Rendering|Components|Light|SetLightColor (Variables|Default|GetPointLight) (Utilities|Struct|MakeLinearColor (Variables|Default|GetR) (Variables|Default|GetG) (Variables|Default|GetB) 0.0) true :!label _label)
    (elif (Utilities|Enum|Equal(Enum) Address "/g")
      (Variables|Default|SetG _returnvalue)
      (goto _label)
      (elif (Utilities|Enum|Equal(Enum) Address "/b")
        (Variables|Default|SetB _returnvalue)
        (goto _label)))))

(event EventBeginPlay)

(event Collision|EventActorBeginOverlap
  (params (OtherActor :type Actor%20Object%20Reference)))

(event EventTick
  (params (DeltaSeconds :type Float%20%28single-precision%29)))

(fn ConstructionScript)