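; BP_OSCIn is a Blueprint that receives OSC messages over the network and rebroadcasts them to other game logic.
; On BeginPlay it creates and stores a listening OSC server on a configurable IP address and port, then binds a message handler.
; The handler extracts each message's full address path and first string argument, prints both, and fires the OnOscReceived dispatcher with them.
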(event Custom|OnMsgReceived
  (params (Message :type OSC%20Message%20Structure%20%28by%20ref%29) (IPAddress :type String) (Port :type Integer))
  (bind _returnvalue (Class|OSCManager|GetOSCMessageAddress Message))
  (bind _returnvalue_2 (Class|OSCManager|GetOSCAddressFullPath _returnvalue))
  (bind _value (Class|OSCManager|GetString Message))
  (Development|PrintString _returnvalue_2)
  (Development|PrintString _value)
  (Default|CallOnOscReceived _returnvalue_2 _value))

(event EventBeginPlay
  (bind _returnvalue (Class|OSCManager|CreateOSCServer (Variables|Default|GetReceive%20IPAddress) (Variables|Default|GetPort) false true "" 0))
  (bind _output_get (Variables|Default|SetOSCServer _returnvalue))
  (EventDispatchers|BindEventtoOnOscMessageReceived _output_get (delegate Custom|OnMsgReceived)))

(event Collision|EventActorBeginOverlap
  (params (OtherActor :type Actor%20Object%20Reference)))

(event EventTick
  (params (DeltaSeconds :type Float%20%28single-precision%29)))

(fn ConstructionScript)